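; Player character Blueprint with a spring-arm camera that turns in yaw steps on the CAMERATEST test input.
; The CameraSweep timeline scales its curve by 90 degrees and adds it to the stored yaw, which updates when each sweep finishes.
; Each finished sweep also advances CurrentNathan, a wrapping index into the four W, A, S, D references stored at BeginPlay.
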(event `self.ReceiveBeginPlay`
  (bind _nathanreferences (`self.NathanReferences`))
  (set `self.InitialCameraRotation` (.rotation (`SceneComponent.GetRelativeTransform` (`self.SpringArm`))))
  (`KismetArrayLibrary.Array_Set` _nathanreferences 0 (`self.W`))
  (`KismetArrayLibrary.Array_Set` _nathanreferences 1 (`self.A`))
  (`KismetArrayLibrary.Array_Set` _nathanreferences 2 (`self.S`))
  (`KismetArrayLibrary.Array_Set` _nathanreferences 3 (`self.D`)))

(event `InputAction|CAMERATEST`
  (params (Key :type "Key Structure"))
  (:`Pressed`
    (bind (_direction _camera_rotation) (`Timeline|CameraSweep` :!via `PlayFromStart`)
      (:`Update`
        (bind _returnvalue (`KismetMathLibrary.ComposeRotators` (`KismetMathLibrary.MakeRotator` 0.0 0.0 (* _camera_rotation 90.0)) (`KismetMathLibrary.MakeRotator` 0.0 0.0 (.yaw (`self.InitialCameraRotation`)))))
        (`SceneComponent.K2_SetWorldRotation` (`self.SpringArm`) _returnvalue false false))
      (:`Finished`
        (set `self.InitialCameraRotation` _returnvalue)
        (`self.SetCurrentNathan` 1)))))

(fn `SetCurrentNathan`
  (params (AmountToAdd :type Integer))
  (bind _returnvalue (+ (`self.CurrentNathan`) AmountToAdd))
  (if (> _returnvalue (- (`KismetArrayLibrary.Array_Length` (`self.NathanReferences`)) 1))
    (set `self.CurrentNathan` 0)
    (elif (< _returnvalue 0)
      (set `self.CurrentNathan` (+ 3 (+ _returnvalue 1)))
      (else
        (set `self.CurrentNathan` _returnvalue)))))

(fn `UserConstructionScript`)