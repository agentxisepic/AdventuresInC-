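; Player controller that forwards movement and sprint input to a movement component, manages the HUD and toggleable inventory, and animates the character with flipbooks.
; Self-recalling Delay loops update the stamina bar and compare sampled pawn positions to set IsMoving.
; Tick selects idle or walking from IsMoving and, on state or side changes, clears all flipbook components and assigns the current side's.
; AddItem stores items through the inventory component, retrying recursively on one result code, and refreshes the UI.
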(event `self.ReceiveBeginPlay`
  (bind _location (.location (`self.GetTransform` (`GameplayStatics.GetPlayerPawn` 0))))
  ;[1 1 1] BeginPlaySetup
  (bind _returnvalue (`|CreateWidget` "/Game/Player/HUD/TESTHUD.TESTHUD_C"))
  (`UserWidget.AddToViewport` _returnvalue 0)
  (bind _returnvalue_2 (`|CreateWidget` "/Game/InventorySystem/UI/Inventory.Inventory_C"))
  (bind _output_get (set `self.InventoryReference` _returnvalue_2))
  (`UserWidget.AddToViewport` _output_get 0)
  (`Widget.SetVisibility` _output_get "Collapsed")
  (set `self.CharacterPositionLast` _location)
  (set `self.CharacterPosition` _location)
  (`self.DetectCharacterMove`)
  (`self.StaminaHandle`))

(event `InputAxis|MoveLeftRight`
  (params (AxisValue :type "Float (single-precision)"))
  ;[1 1 1] Player Movement Handling (Gets Delegated to the Movement Component on the Player)
  (bind _output_get (set `self.DirectionIdentifier` "LR"))
  (`AfflictionMovementComponent.Walk` (`self.GetMovementComponent`) AxisValue _output_get))

(event `InputAction|OpenInventory`
  (params (Key :type "Key Structure"))
  ;[1 1 1] UI Control Handling
  (:`Pressed`
    (bind _isa (`/Engine/EditorBlueprintResources/StandardMacros.FlipFlop`)
      (:`A`
        (`Widget.SetVisibility` (`self.InventoryReference`) "Visible")
        (set `self.bShowMouseCursor` _isa))
      (:`B`
        (`Widget.SetVisibility` (`self.InventoryReference`) "Collapsed")
        (set `self.bShowMouseCursor` _isa)))))

(event `InputAxis|MoveForwardBackward`
  (params (AxisValue :type "Float (single-precision)"))
  ;[1 1 1] Player Movement Handling (Gets Delegated to the Movement Component on the Player)
  (bind _output_get (set `self.DirectionIdentifier` "FB"))
  (`AfflictionMovementComponent.Walk` (`self.GetMovementComponent`) AxisValue _output_get))

(event `InputAxis|Sprint`
  (params (AxisValue :type "Float (single-precision)"))
  ;[1 1 1] Player Movement Handling (Gets Delegated to the Movement Component on the Player)
  (`AfflictionMovementComponent.Sprint` (`self.GetMovementComponent`) AxisValue))

(event `StaminaHandle`
  (bind _returnvalue (`self.GetMovementComponent`))
  ;[1 1 1] Player Movement Handling (Gets Delegated to the Movement Component on the Player)
  (`KismetSystemLibrary.Delay` 0.001)
  (bind _returnvalue_2 (`AfflictionMovementComponent.StaminaHandle` _returnvalue))
  ;[1 1 1] UI Control Handling
  (`/Game/Player/HUD/TESTHUD.UpdateSprintBar` (stale `self.ReceiveBeginPlay` _returnvalue) _returnvalue_2 0.01 _returnvalue)
  (`self.StaminaHandle`))

(event `AddItemToInventory`
  (params (ItemToBeRepresented :type "Item Object Reference"))
  ;[1 1 1] Player Inventory Handling
  (`self.AddItem` (`self.GetInventoryComponent`) (`/Game/InventorySystem/UI/Inventory.InventoryItems` (`self.InventoryReference`)) ItemToBeRepresented))

(event `DetectCharacterMove`
  (bind _location (.location (`self.GetTransform` (`GameplayStatics.GetPlayerPawn` 0))))
  (`KismetSystemLibrary.Delay` 0.1)
  (set `self.CharacterPositionLast` _location)
  (`KismetSystemLibrary.Delay` 0.08)
  (set `self.CharacterPosition` _location)
  (`self.DetectCharacterMove`)
  (if (!= (`self.CharacterPositionLast`) (`self.CharacterPosition`) :`ErrorTolerance` 0.0)
    (set `self.bIsMoving` true)
    (else
      (set `self.bIsMoving` false))))

(event `self.ReceiveTick`
  (params (DeltaSeconds :type "Float (single-precision)"))
  (bind _animation (`self.AnimationStateMachine`))
  (bind _asplayer_character_bp (cast `/Game/Player/PlayerCharacter_BP` (`GameplayStatics.GetPlayerPawn` 0)))
  (bind _currentnathan (`/Game/Player/PlayerCharacter_BP.CurrentNathan` _asplayer_character_bp))
  (if (!= _currentnathan (`self.LastNathanUpdated`))
    (set `self.LastNathanUpdated` _currentnathan)
    (set `self.bNeedsUpdated` true))
  (`self.AssignFlipbook` _animation _currentnathan))

(fn `AddItem`
  (params (InventoryRef :type "Inventory Object Reference (by ref)") (InventoryUIReference :type "/Game/InventorySystem/UI/InventoryItems Object Reference (by ref)") (ItemToBeRepresented :type "Item Object Reference (by ref)"))
  (bind _returnvalue (`Inventory.AddItem` InventoryRef ItemToBeRepresented))
  (if (== _returnvalue -1)
    (`/Game/InventorySystem/UI/InventoryItems.UpdateItemDetails` InventoryUIReference)
    (return)
    (elif (== _returnvalue -2)
      (`/Game/InventorySystem/UI/InventoryItems.UpdateItemDetails` InventoryUIReference)
      (return)
      (elif (== _returnvalue -3)
        (`self.AddItem` InventoryRef InventoryUIReference ItemToBeRepresented)
        (return)
        (else
          (`/Game/InventorySystem/UI/InventoryItems.AddItemToInventory` InventoryUIReference _returnvalue ItemToBeRepresented)
          (`/Game/InventorySystem/UI/InventoryItems.UpdateItemDetails` InventoryUIReference)
          (return))))))

(fn `AnimationStateMachine`
  (returns (Animation :type "/Game/Player/AnimationStates Enum"))
  (cast `/Game/Player/PlayerCharacter_BP` (`GameplayStatics.GetPlayerPawn` 0))
  (if (`self.bIsMoving`)
    (set `self.LastNathanAnimations` "NewEnumerator1")
    (else
      (set `self.LastNathanAnimations` "NewEnumerator0")))
  (if (`|EnumEquality` (`self.NathanAnimations`) (`self.LastNathanAnimations`))
    (set `self.bNeedsUpdated` false)
    (set `self.NathanAnimations` (`self.LastNathanAnimations`))
    (else
      (set `self.bNeedsUpdated` true)
      (set `self.NathanAnimations` (`self.LastNathanAnimations`))))
  (return (`self.LastNathanAnimations`)))

(fn `AssignFlipbook`
  (params (FlipbookName :type "/Game/Player/AnimationStates Enum" :default "NewEnumerator0") (CharacterSide :type Integer))
  (bind (_idolanimations _walkinganimations) (break `/Game/Player/FlipbookStructure` (`self.ArrayOfFlipbooks`)))
  (if (`self.bNeedsUpdated`)
    (bind _asplayer_character_bp (cast `/Game/Player/PlayerCharacter_BP` (`GameplayStatics.GetPlayerPawn` 0)))
    (bind _nathanreferences (`/Game/Player/PlayerCharacter_BP.NathanReferences` _asplayer_character_bp))
    (for _array_element _nathanreferences
      (`PaperFlipbookComponent.SetFlipbook` _array_element null))
    (for (_array_element_2 _array_index) (select `/Game/Player/AnimationStates` FlipbookName :`NewEnumerator0` _idolanimations :`NewEnumerator1` _walkinganimations)
      (if (== _array_index CharacterSide)
        (break)))
    (`PaperFlipbookComponent.SetFlipbook` (`|GetArrayItem` _nathanreferences _array_index) _array_element_2)
    (else
      (return))))

(fn `UserConstructionScript`)